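; BP_InventoryItem is a world pickup actor that the player can add to an inventory.
; On BeginPlay it constructs a BP_BaseItemObject from its image, name, description, count, equipment type and own class, and stores it as its default object reference.
; InteracItem passes that object to the given inventory's AddItemToInventory and destroys the actor only if the add succeeds.
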(event `self.ReceiveBeginPlay`
  (bind _returnvalue (`|GenericCreateObject` self "/Game/Choice/Characters/Inventory/BP_BaseItemObject.BP_BaseItemObject_C" (`self.Image`) (`GameplayStatics.GetObjectClass` self) (`self.Name`) (`self.Description`) (`self.Count`) (`self.EquipmentType`)))
  (set `self.DefoultObjectReference` _returnvalue))

(fn `InteracItem`
  (params (Inventory :type "/Game/Choice/Characters/Inventory/BPC_inventory Object Reference"))
  (bind _add_ (`/Game/Choice/Characters/Inventory/BPC_inventory.AddItemToInventory` Inventory (`self.DefoultObjectReference`)))
  (if _add_
    (`self.K2_DestroyActor`)))

(fn `UserConstructionScript`)