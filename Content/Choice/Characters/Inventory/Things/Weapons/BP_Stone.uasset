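; BP_Stone is a stone weapon projectile that damages what it hits.
; The construction script sets the projectile movement's initial speed from its Speed variable.
; When Base hits an actor, a BadThing is triggered through ActiveThing with the stored main character.
; Any other actor receives MakeDamage with the stored damage and character, but only while the stone is Active.
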(event `self.Base.OnComponentHit`
  (params (HitComponent :type "PrimitiveComponent Object Reference") (OtherActor :type "Actor Object Reference") (OtherComp :type "PrimitiveComponent Object Reference") (NormalImpulse :type "Vector Structure") (Hit :type "HitResult Structure (by ref)"))
  (bind _asbad_thing (cast `/Game/Choice/ActiveThings/BadThing` OtherActor)
    (:`then`
      (`/Game/Choice/ActiveThings/BP_ActiveThings.ActiveThing` _asbad_thing (`self.MainCharacter_0`)))
    (:`CastFailed`
      (if (`self.Active`)
        (`self.MakeDamage` OtherActor (`self.Damage_0`) (`self.MainCharacter_0`))))))

(fn `UserConstructionScript`
  (set `ProjectileMovementComponent.InitialSpeed` (`self.Speed`) (`self.ProjectileMovement`))
  (`parent.UserConstructionScript`))