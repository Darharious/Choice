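; BP_WoodenStick is a wooden stick melee weapon that deals damage through overlap on its Stick component.
; While Active, an overlap either triggers ActiveThing on a BadThing, passing MainCharacter, or stores the actor as Target and calls MakeDamage, intended to spare the wielder.
; Ending any overlap clears Target.
; Construction applies the Simulate flag to physics on Base, then runs the parent script.
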(event `self.ReceiveBeginPlay`
  (`parent.ReceiveBeginPlay`))

(event `self.Stick.OnComponentBeginOverlap`
  (params (OverlappedComponent :type "PrimitiveComponent Object Reference") (OtherActor :type "Actor Object Reference") (OtherComp :type "PrimitiveComponent Object Reference") (OtherBodyIndex :type Integer) (bFromSweep :type Boolean) (SweepResult :type "HitResult Structure (by ref)"))
  ;[1 1 1] При пересечении лезвия(палки), проверяю кому урон нанести. Если пересечение с тем, кто держит палку, ему урона не будет
  (if (`self.Active`)
    (bind _asbad_thing (cast `/Game/Choice/ActiveThings/BadThing` OtherActor)
      (:`then`
        (`/Game/Choice/ActiveThings/BP_ActiveThings.ActiveThing` _asbad_thing (`self.MainCharacter`)))
      (:`CastFailed`
        (bind _output_get (set `self.Target` OtherActor))
        (`self.MakeDamage` _output_get (`self.Damage`) (`self.MainCharacter`))))))

(event `self.Stick.OnComponentEndOverlap`
  (params (OverlappedComponent :type "PrimitiveComponent Object Reference") (OtherActor :type "Actor Object Reference") (OtherComp :type "PrimitiveComponent Object Reference") (OtherBodyIndex :type Integer))
  ;[1 1 1] При пересечении лезвия(палки), проверяю кому урон нанести. Если пересечение с тем, кто держит палку, ему урона не будет
  (set `self.Target` null))

(fn `UserConstructionScript`
  (`PrimitiveComponent.SetSimulatePhysics` (`self.Base`) (`self.Simulate`))
  (`parent.UserConstructionScript`))