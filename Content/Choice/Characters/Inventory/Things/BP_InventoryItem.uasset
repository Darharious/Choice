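; Pickup item actor that goes into a character's inventory and carries shared damage logic.
; On BeginPlay it wraps its properties and class in a BP_BaseItemObject, which InteracItem passes to the inventory, destroying the actor on success.
; MakeDamage adds the attacker's stat damage against living MainCharacter or PB_Nettle targets, skipping the attacker and one team.
; Character hits can spawn a BadThing penalty when the target's team mismatches an enemy-list entry.
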(event `self.ReceiveBeginPlay`
  (bind _returnvalue (`|GenericCreateObject` self "/Game/Choice/Characters/Inventory/Things/BP_BaseItemObject.BP_BaseItemObject_C" (`self.Image`) (`GameplayStatics.GetObjectClass` self) (`self.Name`) (`self.Description`) (`self.Count`) (`self.EquipmentType`)))
  (set `self.DefoultObjectReference` _returnvalue))

(fn `InteracItem`
  (params (Inventory :type "/Game/Choice/Characters/Inventory/BPC_inventory Object Reference"))
  (bind _add_ (`/Game/Choice/Characters/Inventory/BPC_inventory.AddItemToInventory` Inventory (`self.DefoultObjectReference`)))
  (if _add_
    (`self.K2_DestroyActor`)))

(fn `MakeDamage`
  (params (Target :type "Actor Object Reference") (Damage :type "Float (double-precision)") (MainCharacter :type "/Game/Choice/Characters/MainCharacter/MainCharacter Object Reference"))
  (bind _returnvalue (+ (`self.Damage`) (`/Game/Choice/Characters/StatusAC.Damage` (`/Game/Choice/Characters/MainCharacter/MainCharacter.StatusAC` (`self.MainCharacter`)))))
  (bind _output_get (set `self.Target` Target))
  (set `self.Damage` Damage)
  (set `self.MainCharacter` MainCharacter)
  (`/Engine/EditorBlueprintResources/StandardMacros.IsValid` _output_get
    (:`Is Valid`
      (bind _asmain_character (cast `/Game/Choice/Characters/MainCharacter/MainCharacter` _output_get)
        (:`then`
          (if (`|EnumInequality` (`/Game/Choice/Characters/MainCharacter/MainCharacter.Teams` _asmain_character) "NewEnumerator3")
            (bind _output_get_2 (set `self.Target` _asmain_character))
            (if (not (== _output_get_2 (`self.MainCharacter`)))
              (bind _asmain_character_2 (cast `/Game/Choice/Characters/MainCharacter/MainCharacter` (`self.Target`)))
              (if (not (== (`/Game/Choice/Characters/StatusAC.CurrentHP` (`/Game/Choice/Characters/MainCharacter/MainCharacter.StatusAC` _asmain_character_2)) 0.0))
                (`GameplayStatics.ApplyDamage` _asmain_character_2 _returnvalue)
                ;[1 1 1] Накидываю ухудшедние характера, если цель не из списка врагов
                (for _array_element (`/Game/Choice/Characters/MainCharacter/MainCharacter.MyEmemy` (`self.MainCharacter`))
                  (if (not (`|EnumEquality` (`/Game/Choice/Characters/MainCharacter/MainCharacter.Teams` _asmain_character_2) _array_element)) :!label _label
                    (`/Engine/EditorBlueprintResources/StandardMacros.DoOnce` false
                      (:`Completed`
                        (bind _returnvalue_2 (`|SpawnActorFromClass` "/Game/Choice/ActiveThings/BadThing.BadThing_C" (`KismetMathLibrary.MakeTransform` (0.0 0.0 0.0)) "Undefined" "MultiplyWithRoot" null true "NewEnumerator2" -0.1 "Удар по мирному" null))
                        (`/Game/Choice/ActiveThings/BP_ActiveThings.ActiveThing` _returnvalue_2 (`self.MainCharacter`))))))
                (goto _label)))))
        (:`CastFailed`
          (bind _aspb_nettle (cast `/Game/Choice/Characters/MainCharacter/NPC/PB_Nettle` _output_get))
          (if (not (== (`/Game/Choice/Characters/StatusAC.CurrentHP` (`/Game/Choice/Characters/MainCharacter/NPC/PB_Nettle.StatusAC` _aspb_nettle)) 0.0))
            (`GameplayStatics.ApplyDamage` _aspb_nettle _returnvalue)))))))

(fn `UserConstructionScript`)