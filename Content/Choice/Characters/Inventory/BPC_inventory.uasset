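; Inventory component for the main character, handling item storage, equipment slots, the inventory screen and item interaction.
; On BeginPlay it fills inventory and equipment arrays with one shared blank item object, and adding an item replaces the first slot without an item class.
; ToggleInventory creates or removes the player info panel, switching cursor and input mode.
; TraceInteract sphere-traces from the follow camera to cache a target, which Interact messages with the component itself.
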(event `self.ReceiveBeginPlay`
  (bind _returnvalue (`|GenericCreateObject` "/Game/Choice/Characters/Inventory/BP_BaseItemObject.BP_BaseItemObject_C" null null))
  (set `self.DefaultBPBaseItemObject` _returnvalue)
  (`self.InitailizationInventory`)
  (`self.InitializationEquipmentSlot`))

(fn `AddItemToInventory`
  (params (ItemToAdd :type "/Game/Choice/Characters/Inventory/BP_BaseItemObject Object Reference (by ref)"))
  (returns (`Add?` :type Boolean))
  (locals (EmptySlotIndex :type Integer) (`FindEmptySlot?` :type Boolean))
  (bind _ui_inventoryreference (`self.UI_inventoryReference`))
  (for (_array_element _array_index) (`self.Inventory`)
    (`/Engine/EditorBlueprintResources/StandardMacros.IsValid` _array_element
      (:`Is Valid`
        (`|ExecutionSequence`
          (:`then_0`
            (bind _itemreference (`/Game/Choice/Characters/Inventory/BP_BaseItemObject.ItemReference` _array_element))
            (if (`KismetSystemLibrary.IsValidClass` _itemreference)
              (set `local.FindEmptySlot?` false)
              (else
                (set `local.EmptySlotIndex` _array_index)
                (set `local.FindEmptySlot?` true)
                (break))))
          (:`then_1`
            (`KismetSystemLibrary.PrintString` (`KismetSystemLibrary.GetClassDisplayName` _itemreference)))))))
  (if (`local.FindEmptySlot?`)
    (`KismetArrayLibrary.Array_Set` (`self.Inventory`) (`local.EmptySlotIndex`) (`local.ItemToAdd`))
    (`/Engine/EditorBlueprintResources/StandardMacros.IsValid` _ui_inventoryreference
      (:`Is Valid`
        (`/Game/Choice/Characters/Inventory/Widget/UI_InventoryGrid.RefrashInventory` _ui_inventoryreference))
      (:`Is Not Valid`
        _))
    (return true)
    (else
      (`KismetSystemLibrary.PrintString` "Invetory Full")
      (return false))))

(fn `InitailizationInventory`
  (for _ (range (+ (`self.InventorySizw`) 1))
    (`KismetArrayLibrary.Array_Add` (`self.Inventory`) (`self.DefaultBPBaseItemObject`))))

(fn `InitializationEquipmentSlot`
  (for _ (range 8)
    (`KismetArrayLibrary.Array_Add` (`self.EquipmentSlots`) (`self.DefaultBPBaseItemObject`))))

(fn `Interact`
  (bind _currentinteractitem (`self.CurrentInteractItem`)
    (:`then`
      (message `/Game/Choice/Characters/Inventory/BPI_Interact.Interact` _currentinteractitem self))
    (:`else`)))

(fn `ToggleInventory`
  (bind _returnvalue (`GameplayStatics.GetPlayerController` 0))
  (bind _returnvalue_2 (`GameplayStatics.GetPlayerController` 0))
  (bind _ui_inventoryreferencepanel (`self.UI_inventoryReferencePanel`)
    (:`then`
      (`Widget.RemoveFromParent` _ui_inventoryreferencepanel)
      (set `PlayerController.bShowMouseCursor` false _returnvalue)
      (`WidgetBlueprintLibrary.SetInputMode_GameOnly` _returnvalue)
      (set `self.UI_inventoryReferencePanel` null))
    (:`else`
      (`|ExecutionSequence`
        (:`then_0`
          (bind _returnvalue_3 (`|CreateWidget` "/Game/Choice/Characters/Inventory/Widget/UI_PlayerInfoPanel.UI_PlayerInfoPanel_C"))
          (bind _output_get (set `self.UI_inventoryReferencePanel` _returnvalue_3))
          (`UserWidget.AddToViewport` _output_get 0)
          (set `PlayerController.bShowMouseCursor` true _returnvalue_2)
          (`WidgetBlueprintLibrary.SetInputMode_GameAndUIEx` _returnvalue_2 (`self.UI_inventoryReference`) "DoNotLock" true true))))))

(fn `TraceInteract`
  (params (LenghtTrace :type "Float (double-precision)"))
  (bind _followcamera (`/Game/Choice/Characters/MainCharacter/MainCharacter.FollowCamera` (`self.AsMainCharacter`)))
  (bind _returnvalue (`SceneComponent.K2_GetComponentLocation` _followcamera))
  (bind _outhit (`KismetSystemLibrary.SphereTraceSingle` _returnvalue (+ _returnvalue (* (`SceneComponent.GetForwardVector` _followcamera) (`local.LenghtTrace`))) 15.0 "TraceTypeQuery3" false (`|MakeArray` null :!type "Actor Object Reference")))
  (bind (_bblockinghit _binitialoverlap _time _distance _location _impactpoint _normal _impactnormal _physmat _hitactor) (`GameplayStatics.BreakHitResult` _outhit))
  (if _bblockinghit
    (set `self.CurrentInteractItem` _hitactor)
    (else
      (set `self.CurrentInteractItem` null))))