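; BP_PersonalityBad is a one-use interactable with a pulsing point light that changes one of the player's stats.
; A timeline drives the light intensity, flipping between play and reverse each time it finishes.
; Box overlap stores or clears the MainCharacter reference.
; The ActiveThing event switches on TypeThing to upgrade Power, Intelligence, Personality or Endurance through StatusAC by Value, prints its text, then destroys the actor.
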(event `self.ReceiveBeginPlay`
  (bind _output_get (set `self.IsActive` true))
  (if _output_get :!label _label
    (bind (_direction _newtrack_1) (`Timeline|Timeline` :!label _label_2)
      (:`Update`
        (`LightComponent.SetIntensity` (`self.PointLight`) _newtrack_1))
      (:`Finished`
        (set `self.IsActive` (not (`self.IsActive`)))
        (`self.Light`)))
    (else
      (goto _label_2 :!via `Reverse`))))

(event `Light`
  (goto _label))

(event `self.Box.OnComponentBeginOverlap`
  (params (OverlappedComponent :type "PrimitiveComponent Object Reference") (OtherActor :type "Actor Object Reference") (OtherComp :type "PrimitiveComponent Object Reference") (OtherBodyIndex :type Integer) (bFromSweep :type Boolean) (SweepResult :type "HitResult Structure (by ref)"))
  (bind _asmain_character (cast `/Game/Choice/Characters/MainCharacter/MainCharacter` OtherActor))
  (set `self.MainCharacter` _asmain_character))

(event `self.Box.OnComponentEndOverlap`
  (params (OverlappedComponent :type "PrimitiveComponent Object Reference") (OtherActor :type "Actor Object Reference") (OtherComp :type "PrimitiveComponent Object Reference") (OtherBodyIndex :type Integer))
  (set `self.MainCharacter` null))

(event `ActiveThing`
  (switch `/Game/Choice/ActiveThings/E_ActiveTypeThing` (`self.TypeThing`)
    (:`NewEnumerator0`
      (`/Game/Choice/Characters/StatusAC.UpgradePower` (`/Game/Choice/Characters/MainCharacter/MainCharacter.StatusAC` (`self.MainCharacter`)) (`self.Value`)))
    (:`NewEnumerator1`
      (`/Game/Choice/Characters/StatusAC.UpgradeIntelligence` (`/Game/Choice/Characters/MainCharacter/MainCharacter.StatusAC` (`self.MainCharacter`)) (`self.Value`)))
    (:`NewEnumerator2`
      (`/Game/Choice/Characters/StatusAC.UpgradePersonality` (`/Game/Choice/Characters/MainCharacter/MainCharacter.StatusAC` (`self.MainCharacter`)) (`self.Value`)))
    (:`NewEnumerator3`
      (`/Game/Choice/Characters/StatusAC.UpgradeEndurance` (`/Game/Choice/Characters/MainCharacter/MainCharacter.StatusAC` (`self.MainCharacter`)) (`self.Value`))))
  (`KismetSystemLibrary.PrintText` (`self.Text`))
  (`ActorComponent.K2_DestroyComponent` (`self.Box`))
  (`self.K2_DestroyActor`))

(fn `UserConstructionScript`)