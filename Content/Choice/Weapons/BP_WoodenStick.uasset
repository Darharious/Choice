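; BP_WoodenStick is a wooden stick melee weapon that damages characters it touches while active.
; The Stick component's begin overlap stores and prints any MainCharacter other than the wielder as Target, and end overlap clears it.
; When Active, the overlap applies damage to non-wielders, adding half the wielder's StatusAC Power to base Damage.
; The construction script sets physics simulation on Base from the Simulate flag.
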(event `self.Stick.OnComponentBeginOverlap`
  (params (OverlappedComponent :type "PrimitiveComponent Object Reference") (OtherActor :type "Actor Object Reference") (OtherComp :type "PrimitiveComponent Object Reference") (OtherBodyIndex :type Integer) (bFromSweep :type Boolean) (SweepResult :type "HitResult Structure (by ref)"))
  ;[1 1 1] При пересечении лезвия(палки), проверяю кому урон нанести. Если пересечение с тем, кто держит палку, ему урона не будет
  (`|ExecutionSequence`
    (:`then_0`
      (bind _asmain_character (cast `/Game/Choice/Characters/MainCharacter/MainCharacter` OtherActor))
      (if (not (== (`self.MainCharacter`) _asmain_character))
        (bind _output_get (set `self.Target` _asmain_character))
        (`KismetSystemLibrary.PrintString` (`KismetSystemLibrary.GetDisplayName` _output_get))))
    (:`then_1`
      (if (`self.Active`)
        (bind _asmain_character_2 (cast `/Game/Choice/Characters/MainCharacter/MainCharacter` OtherActor))
        (bind _output_get_2 (set `self.Target` _asmain_character_2))
        (if (not (== _output_get_2 (`self.MainCharacter`)))
          (`GameplayStatics.ApplyDamage` (`self.Target`) (+ (`self.Damage`) (* (`/Game/Choice/Characters/StatusAC.Power` (`/Game/Choice/Characters/MainCharacter/MainCharacter.StatusAC` (`self.MainCharacter`))) 0.5))))))))

(event `self.Stick.OnComponentEndOverlap`
  (params (OverlappedComponent :type "PrimitiveComponent Object Reference") (OtherActor :type "Actor Object Reference") (OtherComp :type "PrimitiveComponent Object Reference") (OtherBodyIndex :type Integer))
  ;[1 1 1] При пересечении лезвия(палки), проверяю кому урон нанести. Если пересечение с тем, кто держит палку, ему урона не будет
  (set `self.Target` null))

(fn `UserConstructionScript`
  (`PrimitiveComponent.SetSimulatePhysics` (`self.Base`) (`self.Simulate`))
  (`parent.UserConstructionScript`))