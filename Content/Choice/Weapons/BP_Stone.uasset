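; BP_Stone is a stone weapon that damages a character it hits.
; While Active, a hit on its Base component checks for a MainCharacter other than the stored MainCharacter, skipping any whose HP is zero.
; It applies its own Damage plus the stored character's StatusAC damage, then clears Active so it cannot deal damage again until reactivated.
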(event `self.Base.OnComponentHit`
  (params (HitComponent :type "PrimitiveComponent Object Reference") (OtherActor :type "Actor Object Reference") (OtherComp :type "PrimitiveComponent Object Reference") (NormalImpulse :type "Vector Structure") (Hit :type "HitResult Structure (by ref)"))
  (if (`self.Active`)
    (bind _asmain_character (cast `/Game/Choice/Characters/MainCharacter/MainCharacter` OtherActor))
    (if (== (`self.MainCharacter`) _asmain_character)
      _
      (elif (not (== (`/Game/Choice/Characters/StatusAC.CurrentHP` (`/Game/Choice/Characters/MainCharacter/MainCharacter.StatusAC` _asmain_character)) 0.0))
        (`GameplayStatics.ApplyDamage` _asmain_character (+ (`self.Damage`) (`/Game/Choice/Characters/StatusAC.Damage` (`/Game/Choice/Characters/MainCharacter/MainCharacter.StatusAC` (`self.MainCharacter`)))))
        (set `self.Active` false)))))

(fn `UserConstructionScript`
  (`parent.UserConstructionScript`))